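; BP_AIGecko is a gecko enemy that hurts actors it bumps and explodes when its health runs out.
; Capsule hits trigger effects, apply damage and launch BP_Alice using the gecko's scaled world location, not a direction.
; BeginPlay briefly toggles Attacking after delays, and Wield_Stick can attach a spawned stick to the hand socket.
; Chase, montage and attack-timer logic is disconnected, leaving those events and Tick empty.
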(event OnComponentHit(CapsuleComponent)
  (params (HitComponent :type Primitive%20Component%20Object%20Reference) (OtherActor :type Actor%20Object%20Reference) (OtherComp :type Primitive%20Component%20Object%20Reference) (NormalImpulse :type Vector :default "0, 0, 0") (Hit :type Hit%20Result%20Structure%20%28by%20ref%29))
  (bind _returnvalue (Transformation|GetActorLocation))
  (bind _returnvalue_2 (* _returnvalue 2.0))
  (Utilities|FlowControl|Delay 0.05)
  (Effects|SpawnEmitteratLocation "/Game/StarterContent/Particles/P_Explosion.P_Explosion" (Transformation|GetActorLocation))
  (Audio|PlaySoundatLocation (Variables|Default|Getimpact%20sound) "0, 0, 0" "0, 0, 0" 1.0 1.0 0.0 0 0 0 0)
  (Actor|GetActorOfClass "/Game/ThirdPerson/Blueprints/BP_Alice.BP_Alice_C")
  (Game|Damage|ApplyDamage OtherActor 1.0 0 0)
  (bind _asbp_alice (Utilities|Casting|CastToBP_Alice OtherActor))
  (Character|LaunchCharacter _asbp_alice (Math|Vector|MakeVector (.x _returnvalue_2) (.y _returnvalue_2) (+ (.z _returnvalue_2) 5e+01)) false false))

(event Custom|attack\)

(event Custom|chae%20player)

(event Custom|pusing)

(event Custom|Wield_Stick
  (bind _returnvalue (Game|SpawnActorfromClass "/Game/ThirdPerson/Blueprints/BP_Stick.BP_Stick_C" (Transformation|GetActorTransform) "Undefined" "MultiplyWithRoot" 0 0))
  (Transformation|AttachComponentToComponent _returnvalue (Variables|Character|GetMesh) "hand_r_stick_Socket" "SnapToTarget" "SnapToTarget" "SnapToTarget" true))

(event Game|Damage|EventAnyDamage
  (params (Damage :type Float%20%28single-precision%29) (DamageType :type Damage%20Type%20Object%20Reference) (InstigatedBy :type Controller%20Object%20Reference) (DamageCauser :type Actor%20Object%20Reference))
  (Development|PrintString "kena geko")
  (bind _output_get (Variables|Default|SetHealth (- (Variables|Default|GetHealth) Damage)))
  (Development|PrintString (Utilities|String|ToString(Float) _output_get))
  (if (<= (Variables|Default|GetHealth) 0.0)
    (Effects|SpawnEmitteratLocation "/Game/StarterContent/Particles/P_Explosion.P_Explosion" (Transformation|GetActorLocation))
    (Actor|DestroyActor)))

(event EventTick
  (params (DeltaSeconds :type Float%20%28single-precision%29)))

(event EventBeginPlay
  (Utilities|FlowControl|Delay 5.0)
  (Variables|Default|SetAttacking true)
  (Utilities|FlowControl|Delay 5.0)
  (Variables|Default|SetAttacking false))

(fn ConstructionScript)