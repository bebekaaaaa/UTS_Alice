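; BP_batubegokduar is a destructible rock actor ("batu") that explodes when its health runs out.
; An overlap with another actor makes the Batu component visible.
; Any damage is subtracted from Health with debug prints; at zero or below it spawns an enlarged P_Explosion emitter at its location and destroys itself.
; An unconnected SpawnActor node with fixed coordinates is left in the graph and never runs.
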(event EventBeginPlay)

(event Collision|EventActorBeginOverlap
  (params (OtherActor :type Actor%20Object%20Reference))
  (Rendering|SetVisibility (Variables|Default|Getbatu) true false))

(event Game|Damage|EventAnyDamage
  (params (Damage :type Float%20%28single-precision%29) (DamageType :type Damage%20Type%20Object%20Reference) (InstigatedBy :type Controller%20Object%20Reference) (DamageCauser :type Actor%20Object%20Reference))
  (Development|PrintString "kena batu")
  (bind _output_get (Variables|Default|SetHealth (- (Variables|Default|GetHealth) Damage)))
  (Development|PrintString (Utilities|String|ToString(Float) _output_get))
  (if (<= (Variables|Default|GetHealth) 0.0)
    (Effects|SpawnEmitteratLocation "/Game/StarterContent/Particles/P_Explosion.P_Explosion" (Transformation|GetActorLocation) "0, 0, 0" "4.000000,4.000000,4.000000")
    (Actor|DestroyActor)))

(event EventTick
  (params (DeltaSeconds :type Float%20%28single-precision%29)))

(fn ConstructionScript)