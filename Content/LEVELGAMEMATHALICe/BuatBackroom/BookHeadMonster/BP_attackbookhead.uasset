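; Projectile attack for the BookHead monster that damages whatever it hits.
; On BeginPlay it explicitly keeps collision with its instigator (or owner) enabled, then aims its velocity once at a valid Target, without homing.
; On box hit it forwards the hit actor through an impact callback, plays the impact effect and sound, applies damage and destroys itself.
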(event OnComponentHit(BoxCollision)
  (params (HitComponent :type Primitive%20Component%20Object%20Reference) (OtherActor :type Actor%20Object%20Reference) (OtherComp :type Primitive%20Component%20Object%20Reference) (NormalImpulse :type Vector :default "0, 0, 0") (Hit :type Hit%20Result%20Structure%20%28by%20ref%29))
  (bind _location (Collision|BreakHitResult Hit))
  (Default|CallOnProjectileImpact (Variables|Default|GetTarget_0) OtherActor)
  (Niagara|SpawnSystematLocation (Variables|Default|Getimpact%20effect) _location)
  (Audio|PlaySoundatLocation (Variables|Default|Getimpact%20sound) _location "0, 0, 0" 1.0 1.0 0.0 0 0 0 0)
  (Game|Damage|ApplyDamage OtherActor 1.0 0 0)
  (Actor|DestroyActor))

(event Custom|RotateToTarget
  (Variables|/Script/Engine.MovementComponent|SetVelocity (Variables|Default|GetProjectileMovement) (* (Math|Vector|GetUnitDirection(Vector) (Transformation|GetActorLocation) (Transformation|GetActorLocation (Variables|Default|GetTarget))) (Variables|Default|GetSpeed))))

(event Collision|EventActorBeginOverlap
  (params (OtherActor :type Actor%20Object%20Reference)))

(event EventTick
  (params (DeltaSeconds :type Float%20%28single-precision%29)))

(event EventBeginPlay
  (bind _returnvalue (Game|GetInstigator))
  (Collision|IgnoreActorwhenMoving (Variables|Default|GetBox%20Collision) (select (Utilities|IsValid _returnvalue) _returnvalue (Components|GetOwner)) false)
  (Variables|Default|GetTarget
    (:then
      (CallFunction|RotatetoTarget))
    (:else)))

(fn ConstructionScript)

(fn RotatetoTarget)