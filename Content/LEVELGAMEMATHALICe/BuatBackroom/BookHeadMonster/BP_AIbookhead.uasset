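; BP_AIbookhead is the Bookhead monster, an enemy that fires projectiles at BP_Alice.
; Its Attack event spawns a projectile at its shoot point with Alice as target, plays the attack montage, and calls Bookheademboh on completion.
; Any damage lowers Health with debug prints; at zero it spawns an explosion, plays a sound and destroys itself.
; Sphere overlap events are empty, and several older attack fragments are disconnected.
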(event OnComponentBeginOverlap(Sphere)
  (params (OverlappedComponent :type Primitive%20Component%20Object%20Reference) (OtherActor :type Actor%20Object%20Reference) (OtherComp :type Primitive%20Component%20Object%20Reference) (OtherBodyIndex :type Integer) (bFromSweep :type Boolean) (SweepResult :type Hit%20Result%20Structure%20%28by%20ref%29)))

(event OnComponentEndOverlap(Sphere)
  (params (OverlappedComponent :type Primitive%20Component%20Object%20Reference) (OtherActor :type Actor%20Object%20Reference) (OtherComp :type Primitive%20Component%20Object%20Reference) (OtherBodyIndex :type Integer)))

(event Custom|Attack
  (bind _returnvalue (Actor|GetActorOfClass "/Game/ThirdPerson/Blueprints/BP_Alice.BP_Alice_C"))
  (Game|SpawnActorfromClass (Variables|Default|Getprojectile%20type) (Transformation|GetWorldTransform (Variables|Default|GetShootPointt)) "Undefined" "MultiplyWithRoot" self 0.0 1e+03 _returnvalue false 0)
  (Animation|Montage|PlayMontage (Variables|Character|GetMesh) "/Game/LEVELGAMEMATHALICe/BuatBackroom/BookHeadMonster/Demo/Animations/AM_bookheadattack.AM_bookheadattack"
    (:OnCompleted
      (Default|CallBookheademboh))))

(event EventBeginPlay)

(event Game|Damage|EventAnyDamage
  (params (Damage :type Float%20%28single-precision%29) (DamageType :type Damage%20Type%20Object%20Reference) (InstigatedBy :type Controller%20Object%20Reference) (DamageCauser :type Actor%20Object%20Reference))
  (bind _returnvalue (Transformation|GetActorLocation))
  (Development|PrintString "kena boss")
  (bind _output_get (Variables|Default|SetHealth (- (Variables|Default|GetHealth) Damage)))
  (Development|PrintString (Utilities|String|ToString(Float) _output_get))
  (if (<= (Variables|Default|GetHealth) 0.0)
    (Effects|SpawnEmitteratLocation "/Game/StarterContent/Particles/P_Explosion.P_Explosion" _returnvalue)
    (Audio|PlaySoundatLocation "/Game/LEVELGAMEMATHALICe/BuatBackroom/BookHeadMonster/bookhead_modyarrr.bookhead_modyarrr" _returnvalue "0, 0, 0" 1.0 1.0 0.0 0 0 0 0)
    (Actor|DestroyActor)))

(fn ConstructionScript)