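; BP_platform4 is a one-shot trigger actor that spawns a BP_AIbookhead when something overlaps it.
; Any actor overlap fires the spawn with no filtering, then the blueprint destroys itself and prints a debug string.
; Timeline-driven mesh movement and a mesh rotation node remain in the graph but are unconnected, so the platform never animates.
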(event EventBeginPlay)

(event Collision|EventActorBeginOverlap
  (params (OtherActor :type Actor%20Object%20Reference))
  (Game|SpawnActorfromClass "/Game/LEVELGAMEMATHALICe/BuatBackroom/BookHeadMonster/BP_AIbookhead.BP_AIbookhead_C" (Math|Transform|MakeTransform "0, 0, 0" "0, 0, 0" "1.000000,1.000000,1.000000") "Undefined" "MultiplyWithRoot" 0 0)
  (Actor|DestroyActor)
  (Development|PrintText "asu"))

(event EventTick
  (params (DeltaSeconds :type Float%20%28single-precision%29)))

(fn ConstructionScript)