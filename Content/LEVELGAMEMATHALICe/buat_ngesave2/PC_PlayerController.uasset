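; Player controller that provides debug hotkeys for testing the global player health and save system.
; Debug key presses cast the game instance to GI_GlobalVariable, then raise or lower its Health by one, or call SaveFile and print a confirmation string.
; BeginPlay, Tick and the construction script are empty.
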(event EventBeginPlay)

(event EventTick
  (params (DeltaSeconds :type Float%20%28single-precision%29)))

(event Input|KeyboardEvents|DebugKey3
  (params (Key :type Key%20Structure :default "None") (ActionValue :type Input%20Action%20Value%20Structure))
  (:Pressed
    (bind _asgi_global_variable (Utilities|Casting|CastToGI_GlobalVariable (Game|GetGameInstance)))
    (Math|Integer|IncrementInt (Variables|/Game/LEVELGAMEMATHALICe/buat_ngesave2/GI_GlobalVariable.GI_GlobalVariable_C|Gethealth _asgi_global_variable))))

(event Input|KeyboardEvents|DebugKey4
  (params (Key :type Key%20Structure :default "None") (ActionValue :type Input%20Action%20Value%20Structure))
  (:Pressed
    (bind _asgi_global_variable (Utilities|Casting|CastToGI_GlobalVariable (Game|GetGameInstance)))
    (Math|Integer|DecrementInt (Variables|/Game/LEVELGAMEMATHALICe/buat_ngesave2/GI_GlobalVariable.GI_GlobalVariable_C|Gethealth _asgi_global_variable))))

(event Input|KeyboardEvents|DebugKey6
  (params (Key :type Key%20Structure :default "None") (ActionValue :type Input%20Action%20Value%20Structure))
  (:Pressed
    (bind _asgi_global_variable (Utilities|Casting|CastToGI_GlobalVariable (Game|GetGameInstance)))
    (Default|SaveFile _asgi_global_variable)
    (Development|PrintString "Hello")))

(fn ConstructionScript)