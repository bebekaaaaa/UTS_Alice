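; Base projectile Blueprint that flies at an optional target, damages what it hits, then destroys itself.
; The construction script applies speed and gravity to ProjectileMovement and enables homing on the target's root component when requested.
; On BeginPlay it ignores its instigator, or owner as fallback, and aims velocity at any valid target.
; A box collision hit fires the OnProjectileImpact dispatcher, impact effect, sound and fixed damage.
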(event OnComponentHit(BoxCollision)
  (params (HitComponent :type Primitive%20Component%20Object%20Reference) (OtherActor :type Actor%20Object%20Reference) (OtherComp :type Primitive%20Component%20Object%20Reference) (NormalImpulse :type Vector :default "0, 0, 0") (Hit :type Hit%20Result%20Structure%20%28by%20ref%29))
  (bind _location (Collision|BreakHitResult Hit))
  (Default|CallOnProjectileImpact OtherActor Hit)
  (Niagara|SpawnSystematLocation (Variables|effect|Getimpact%20effect) _location)
  (Audio|PlaySoundatLocation (Variables|effect|Getimpact%20sound) _location "0, 0, 0" 1.0 1.0 0.0 0 0 0 0)
  (Game|Damage|ApplyDamage OtherActor 1.0 0 0)
  (Actor|DestroyActor))

(event Custom|Rotate%20to%20Target
  (Variables|/Script/Engine.MovementComponent|SetVelocity (Variables|Default|GetProjectileMovement) (* (Math|Vector|GetUnitDirection(Vector) (Transformation|GetActorLocation) (Transformation|GetActorLocation (Variables|Default|GetTarget))) (Variables|ProjectileSetting|GetSpeed))))

(event EventBeginPlay
  (bind _returnvalue (Game|GetInstigator))
  (Collision|IgnoreActorwhenMoving (Variables|Default|GetBox%20Collision) (select (Utilities|IsValid _returnvalue) _returnvalue (Components|GetOwner)) true)
  (Variables|Default|GetTarget
    (:then
      (CallFunction|RotatetoTarget))
    (:else)))

(fn ConstructionScript
  (bind _projectilemovement (Variables|Default|GetProjectileMovement))
  (Variables|/Script/Engine.ProjectileMovementComponent|SetInitialSpeed _projectilemovement (Variables|ProjectileSetting|GetSpeed))
  (Variables|/Script/Engine.ProjectileMovementComponent|SetMaxSpeed _projectilemovement (Variables|ProjectileSetting|GetSpeed))
  (Variables|/Script/Engine.ProjectileMovementComponent|SetProjectileGravityScale _projectilemovement (Variables|ProjectileSetting|GetGravity))
  (Variables|Default|GetTarget
    (:then
      (if (Variables|Default|Getis%20Homing)
        (Variables|/Script/Engine.ProjectileMovementComponent|SetbIsHomingProjectile _projectilemovement true)
        (Variables|/Script/Engine.ProjectileMovementComponent|SetHomingTargetComponent _projectilemovement (Variables|/Script/Engine.Actor|GetRootComponent (Variables|Default|GetTarget)))))
    (:else)))