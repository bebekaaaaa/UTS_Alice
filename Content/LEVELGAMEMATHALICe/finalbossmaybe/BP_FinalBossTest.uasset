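; BP_FinalBossTest is a test final boss character that fires projectiles targeted at BP_Alice.
; A looping timer spawns a randomly chosen lightning-arrow or green-shuriken projectile at ShootPoint, while a separate Attack event plays a melee-style montage guarded by an Attacking flag.
; BeginPlay hands itself to its WB_healthboss widget; AnyDamage lowers Health and, at zero, plays a montage, then explodes and destroys the boss.
; Stick-wielding logic is present but disconnected.
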(event Custom|Shoot
  (bind _returnvalue (Game|GetInstigator))
  (bind _returnvalue_2 (Actor|GetActorOfClass "/Game/ThirdPerson/Blueprints/BP_Alice.BP_Alice_C"))
  (bind _returnvalue_3 (Game|SpawnActorfromClass (Utilities|Select :Index (Math|Random|RandomInteger 2) :Option%200 "/Game/LEVELGAMEMATHALICe/finalbossmaybe/BP_ProjectileBase_panahPetir.BP_ProjectileBase_panahPetir_C" :Option%201 "/Game/LEVELGAMEMATHALICe/finalbossmaybe/BP_ProjectileBase_shurikenHijau.BP_ProjectileBase_shurikenHijau_C") (Transformation|GetWorldTransform (Variables|Default|GetShoot%20point)) "Undefined" "MultiplyWithRoot" self 0.0 1e+03 _returnvalue_2 false 0))
  (Development|PrintString "attack")
  (Collision|IgnoreActorwhenMoving (Variables|Collision|GetCapsuleComponent) 0 true)
  (Collision|IgnoreActorwhenMoving (Variables|/Game/LEVELGAMEMATHALICe/finalbossmaybe/BP_ProjectileBase.BP_ProjectileBase_C|GetBox%20Collision _returnvalue_3) (select (Utilities|IsValid _returnvalue) _returnvalue (Components|GetOwner)) true))

(event Custom|Wield_Stick)

(event Custom|Attack
  (if (not (Variables|Default|Getattacking))
    (Variables|Default|Setattacking true)
    (Animation|Montage|PlayMontage (Variables|Character|GetMesh) "/Game/ThirdPerson/Blueprints/AnimasineAlice/attack/attack1/AM_attack1.AM_attack1" 1.0 0.0 "None" false
      (:OnCompleted
        ;[0.15 0.15 0.15 0.5] reset
        (Variables|Default|Setattacking false)))))

(event Game|Damage|EventAnyDamage
  (params (Damage :type Float%20%28single-precision%29) (DamageType :type Damage%20Type%20Object%20Reference) (InstigatedBy :type Controller%20Object%20Reference) (DamageCauser :type Actor%20Object%20Reference))
  (Development|PrintString "kena boss")
  (bind _output_get (Variables|Default|SetHealth (- (Variables|Default|GetHealth) Damage)))
  (Development|PrintString (Utilities|String|ToString(Float) _output_get))
  (if (<= (Variables|Default|GetHealth) 0.0)
    (Animation|Montage|PlayMontage (Variables|Character|GetMesh) "/Game/LEVELGAMEMATHALICe/finalbossmaybe/AM_mbengok.AM_mbengok"
      (:OnCompleted
        (Effects|SpawnEmitteratLocation "/Game/StarterContent/Particles/P_Explosion.P_Explosion" (Transformation|GetActorLocation))
        (Actor|DestroyActor)))))

(event EventBeginPlay
  (Utilities|Time|SetTimerbyEvent (delegate Custom|Shoot) (Variables|Default|GetFrequency) true)
  (bind _aswb_healthboss (Utilities|Casting|CastToWB_healthboss (UserInterface|GetWidget (Variables|Default|GetWidget))))
  (Variables|Default|SetAs%20WB%20Healthboss _aswb_healthboss)
  (Variables|/Game/LEVELGAMEMATHALICe/finalbossmaybe/WB_healthboss.WB_healthboss_C|SetAs%20BP%20Final%20Boss%20Test _aswb_healthboss self))

(fn ConstructionScript)