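; BP_ProjectileShooter is a destructible turret-like actor that periodically fires projectiles targeting BP_Alice.
; A looping timer spawns the configurable projectile type at ShootPoint, passing Alice as Target.
; Each projectile's collision box ignores the shooter's instigator, or its owner as fallback.
; Damage sets health to damage minus current health (reversed subtraction), clamped, and at zero the actor explodes and destroys itself.
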(event Custom|Shoot
  (bind _returnvalue (Game|GetInstigator))
  (bind _returnvalue_2 (Actor|GetActorOfClass "/Game/ThirdPerson/Blueprints/BP_Alice.BP_Alice_C"))
  (bind _returnvalue_3 (Game|SpawnActorfromClass (Variables|Default|Getprojectile%20type) (Transformation|GetWorldTransform (Variables|Default|GetShootPoint)) "Undefined" "MultiplyWithRoot" self 0.0 1e+03 _returnvalue_2 false 0))
  (Collision|IgnoreActorwhenMoving (Variables|Default|GetCapsule) 0 true)
  (Collision|IgnoreActorwhenMoving (Variables|/Game/LEVELGAMEMATHALICe/finalbossmaybe/BP_ProjectileBase.BP_ProjectileBase_C|GetBox%20Collision _returnvalue_3) (select (Utilities|IsValid _returnvalue) _returnvalue (Components|GetOwner)) true))

(event EventBeginPlay
  (Utilities|Time|SetTimerbyEvent (delegate Custom|Shoot) (Variables|Default|GetFrequency) true))

(event Game|Damage|EventAnyDamage
  (params (Damage :type Float%20%28single-precision%29) (DamageType :type Damage%20Type%20Object%20Reference) (InstigatedBy :type Controller%20Object%20Reference) (DamageCauser :type Actor%20Object%20Reference))
  (Variables|Default|Setheatlh (Math|Float|Clamp(Float) (- Damage (Variables|Default|Getheatlh)) 0.0 5.0))
  (if (<= (Variables|Default|Getheatlh) 0.0)
    (Effects|SpawnEmitteratLocation "/Game/StarterContent/Particles/P_Explosion.P_Explosion" "0, 0, 0")
    (Actor|DestroyActor)))

(fn ConstructionScript)