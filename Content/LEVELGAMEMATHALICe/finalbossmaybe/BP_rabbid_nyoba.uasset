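; Rabbit boss character, apparently a final-boss prototype, that shoots at Alice and has a health bar widget.
; A looping timer fires one of two random projectiles from Slap1, targeted at BP_Alice.
; Attack plays a montage with a notify-triggered scream, guarded against overlap.
; Damage lowers clamped health, with death playing animation and sound before a delayed explosion and destroy; contact damage and knockback logic is unwired.
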(event OnComponentHit(slap1)
  (params (HitComponent :type Primitive%20Component%20Object%20Reference) (OtherActor :type Actor%20Object%20Reference) (OtherComp :type Primitive%20Component%20Object%20Reference) (NormalImpulse :type Vector :default "0, 0, 0") (Hit :type Hit%20Result%20Structure%20%28by%20ref%29)))

(event Custom|Shoot
  (bind _returnvalue (Game|GetInstigator))
  ;[0.15 0.15 0.15 0.5] Comment
  (bind _returnvalue_2 (Actor|GetActorOfClass "/Game/ThirdPerson/Blueprints/BP_Alice.BP_Alice_C"))
  (bind _returnvalue_3 (Game|SpawnActorfromClass (Utilities|Select :Index (Math|Random|RandomInteger 2) :Option%200 "/Game/LEVELGAMEMATHALICe/finalbossmaybe/BP_ProjectileBase_panahPetir.BP_ProjectileBase_panahPetir_C" :Option%201 "/Game/LEVELGAMEMATHALICe/finalbossmaybe/BP_ProjectileBase_shurikenHijau.BP_ProjectileBase_shurikenHijau_C") (Transformation|GetWorldTransform (Variables|Default|Getslap1)) "Undefined" "MultiplyWithRoot" self 0.0 1e+03 _returnvalue_2 false 0))
  (Collision|IgnoreActorwhenMoving (Variables|Collision|GetCapsuleComponent) 0 true)
  (Collision|IgnoreActorwhenMoving (Variables|/Game/LEVELGAMEMATHALICe/finalbossmaybe/BP_ProjectileBase.BP_ProjectileBase_C|GetBox%20Collision _returnvalue_3) (select (Utilities|IsValid _returnvalue) _returnvalue (Components|GetOwner)) true))

(event Custom|Attack
  (if (> (Variables|Default|GetHealth) 0.0)
    (if (not (Variables|Default|Getattacking))
      (Variables|Default|Setattacking true)
      (Animation|Montage|PlayMontage (Variables|Character|GetMesh) "/Game/LEVELGAMEMATHALICe/finalbossmaybe/AM_lawan.AM_lawan" 1.0 0.0 "None" false
        (:OnCompleted
          ;[0.15 0.15 0.15 0.5] reset
          (Variables|Default|Setattacking false))
        (:OnNotifyBegin
          (Audio|PlaySoundatLocation "/Game/_GENERATED/arnet/RabbitTeriak.RabbitTeriak" "0, 0, 0" "0, 0, 0" 0.5 1.0 0.0 0 0 0 0))))
    (else
      (Variables|Default|SetAttacking false))))

(event Game|Damage|EventAnyDamage
  (params (Damage :type Float%20%28single-precision%29) (DamageType :type Damage%20Type%20Object%20Reference) (InstigatedBy :type Controller%20Object%20Reference) (DamageCauser :type Actor%20Object%20Reference))
  (bind _returnvalue (Transformation|GetActorLocation))
  (bind _output_get (Variables|Default|SetHealth (Math|Float|Clamp(Float) (- (Variables|Default|GetHealth) Damage) 0.0 5.0)))
  (Development|PrintString (Utilities|String|ToString(Float) _output_get))
  (if (<= (Variables|Default|GetHealth) 0.0)
    (Components|Movement|StopMovementImmediately (Variables|Character|GetCharacterMovement))
    (Animation|PlayAnimMontage "/Game/LEVELGAMEMATHALICe/finalbossmaybe/AM_mbengok.AM_mbengok" 1.0 "None")
    (Audio|PlaySoundatLocation "/Game/LEVELGAMEMATHALICe/finalbossmaybe/Sucipto_mbengok.Sucipto_mbengok" _returnvalue "0, 0, 0" 2.0 1.0 0.0 0 0 0 0)
    (Utilities|FlowControl|Delay 1e+01)
    (Effects|SpawnEmitteratLocation "/Game/StarterContent/Particles/P_Explosion.P_Explosion" _returnvalue)
    (Actor|DestroyActor)))

(event EventBeginPlay
  (Utilities|Time|SetTimerbyEvent (delegate Custom|Shoot) (Variables|Default|GetFrequency) true)
  (bind _aswb_healthboss (Utilities|Casting|CastToWB_healthboss (UserInterface|GetWidget (Variables|Default|GetWidget))))
  (Variables|Default|SetAs%20WB%20Healthboss _aswb_healthboss)
  (Variables|/Game/LEVELGAMEMATHALICe/finalbossmaybe/WB_healthboss.WB_healthboss_C|SetAs%20BP%20Final%20Boss%20Test _aswb_healthboss 0))

(fn ConstructionScript)