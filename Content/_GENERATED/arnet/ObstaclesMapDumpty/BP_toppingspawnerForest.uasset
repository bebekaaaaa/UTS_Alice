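; Spawner actor that continuously drops random topping actors across an area, likely for a forest obstacle map.
; Tick feeds a one-second Delay, so about once per second it spawns a random class from the Toppingclass array.
; Each spawn lands at a random X/Y within the Box extent around the actor, at the actor's height.
; Counter-limited spawning, debug print and topping cleanup logic are left unconnected and never run.
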(event Collision|EventActorBeginOverlap
  (params (OtherActor :type Actor%20Object%20Reference)))

(event EventTick
  (params (DeltaSeconds :type Float%20%28single-precision%29))
  (bind _returnvalue (Transformation|GetActorLocation))
  (bind _box (Variables|Default|GetBox))
  (bind _boxextent (Variables|/Script/Engine.BoxComponent|GetBoxExtent _box))
  (Utilities|FlowControl|Delay 1.0)
  (Game|SpawnActorfromClass (.OutItem (Utilities|Array|Random (Variables|Default|Gettoppingclass))) (Math|Transform|MakeTransform (Math|Vector|MakeVector (Math|Random|RandomFloatinRange (- (.x _returnvalue) (.x _boxextent)) (+ (.x _returnvalue) (.x _boxextent))) (Math|Random|RandomFloatinRange (- (.y _returnvalue) (.y _boxextent)) (+ (.y _returnvalue) (.y _boxextent))) (.z _returnvalue)) "0, 0, 0" "1.000000,1.000000,1.000000") "Undefined" "MultiplyWithRoot" 0 0))

(fn ConstructionScript)